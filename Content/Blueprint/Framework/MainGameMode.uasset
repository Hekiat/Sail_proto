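; MainGameMode is the game mode for a turn-based game where the player's turn runs as threads of functions such as move, shield and ranged attack.
; On begin play it finds the LevelManager, spawns the default owned functions and creates a main thread tied to the player character.
; PlayTurn runs threads sequentially through end-of-play callbacks, then a turn-ended dispatcher notifies every thread and function.
; It also tracks the selected function and broadcasts selection changes.
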(event Custom|Event%20Play%20Turn
  (CallFunction|ClearSelection)
  (Development|PrintString "Play Turn")
  (Variables|GameFlow|SetIsPlaying true)
  (CallFunction|PlayThread))

(event Custom|TurnEndedDispatcher_Event
  (for _array_element (Variables|Default|GetThreadList)
    (Default|EventEndTurn _array_element))
  (for _array_element_2 (Variables|Default|GetOwnedFunctions)
    (Default|EventEndTurn _array_element_2)))

(event EventBeginPlay
  (bind _outactors (Actor|GetAllActorsOfClass "/Game/Blueprint/LevelManager.LevelManager_C"))
  (Variables|Default|SetLevelManager (Utilities|Array|Get(acopy) _outactors))
  (CallFunction|BuildDefaultFunction)
  (bind _asmain_character_bp (Utilities|Casting|CastToMainCharacterBP (Game|Player|GetPlayerPawn 0)))
  (bind _output_get (Variables|Default|SetMainCharacter _asmain_character_bp))
  (bind _returnvalue (Game|SpawnActorfromClass "/Game/Blueprint/FunctionActors/ThreadBP.ThreadBP_C" (Math|Transform|MakeTransform "0, 0, 0" "0, 0, 0" "1,1,1") "Undefined" 0 "Main" 0 6 _output_get 0))
  (Utilities|Array|Add (Variables|Default|GetThreadList) _returnvalue)
  (EventDispatchers|BindEventtoTurnEndedDispatcher (delegate Custom|TurnEndedDispatcher_Event)))

(event EventTick
  (params (DeltaSeconds :type Float%20%28single-precision%29)))

(fn ConstructionScript)

(fn BuildDefaultFunction
  (Utilities|FlowControl|Sequence
    (:then_0
      (Utilities|FlowControl|ForLoopwithBreak 0 2
        (:LoopBody
          (bind _returnvalue (Game|SpawnActorfromClass "/Game/Blueprint/FunctionActors/Function_MoveBP.Function_MoveBP_C" (Math|Transform|MakeTransform "0, 0, 0") "Undefined" 0 0 2 0))
          (Utilities|Array|Add (Variables|Default|GetOwnedFunctions) _returnvalue))))
    (:then_1
      (bind _returnvalue_2 (Game|SpawnActorfromClass "/Game/Blueprint/FunctionActors/Function_ShieldBP.Function_ShieldBP_C" (Math|Transform|MakeTransform "0, 0, 0" "0, 0, 0" "1,1,1") "Undefined" 0 0 2 0))
      (Utilities|Array|Add (Variables|Default|GetOwnedFunctions) _returnvalue_2))
    (:then_2
      (bind _returnvalue_3 (Game|SpawnActorfromClass "/Game/Blueprint/FunctionActors/Function_RangeAttackBP.Function_RangeAttackBP_C" (Math|Transform|MakeTransform "0, 0, 0" "0, 0, 0" "1,1,1") "Undefined" 0 0 1 0))
      (Utilities|Array|Add (Variables|Default|GetOwnedFunctions) _returnvalue_3))))

(fn SelectFunction
  (params (Function :type Function%20Base%20BP%20Object%20Reference))
  (Utilities|IsValid (Variables|Default|GetSelectedFunction)
    (:Is%20Valid
      (Default|SetSelected (Variables|Default|GetSelectedFunction) false))
    (:Is%20Not%20Valid
      _))
  (bind _output_get (Variables|Default|SetSelectedFunction Function))
  (Default|SetSelected _output_get true)
  (Default|CallFunctionSelectionChangedDispatcher))

(fn PlayThread
  (params (ThreadID :type Integer))
  (bind _threadlist (Variables|Default|GetThreadList))
  (if (Utilities|Array|IsValidIndex _threadlist (Variables|GameFlow|GetPlayingThreadID))
    (EventDispatchers|UnbindallEventsfromOnPlayEnded (Utilities|Array|Get(acopy) _threadlist (Variables|GameFlow|GetPlayingThreadID))))
  (bind _output_get (Variables|GameFlow|SetPlayingThreadID ThreadID))
  (EventDispatchers|BindEventtoOnPlayEnded (Utilities|Array|Get(acopy) (Variables|Default|GetThreadList) _output_get) (EventDispatchers|CreateEvent :!event OnThreadPlayEnded))
  (Default|StartPlay (Utilities|Array|Get(acopy) (Variables|Default|GetThreadList) _output_get)))

(fn OnThreadPlayEnded
  (EventDispatchers|UnbindallEventsfromOnPlayEnded (Utilities|Array|Get(acopy) (Variables|Default|GetThreadList) (Variables|GameFlow|GetPlayingThreadID)))
  (if (== (Variables|GameFlow|GetPlayingThreadID) (Utilities|Array|LastIndex (Variables|Default|GetThreadList)))
    ;[1 1 1] Last Thread, end of the turn
    (Variables|GameFlow|SetIsPlaying false)
    (Variables|GameFlow|SetPlayingThreadID -1)
    (Default|CallTurnEndedDispatcher)
    (else
      ;[1 1 1] Play Next Thread
      (bind _result (Math|Integer|IncrementInt (Variables|GameFlow|GetPlayingThreadID))
        (:%20%20
          (CallFunction|PlayThread _result)
          (Development|PrintString "Plqy Next Thread"))))))

(fn ClearSelection
  (Utilities|IsValid (Variables|Default|GetSelectedFunction)
    (:Is%20Valid
      (Default|SetSelected (Variables|Default|GetSelectedFunction) false))
    (:Is%20Not%20Valid
      _))
  (Variables|Default|SetSelectedFunction 0)
  (Default|CallFunctionSelectionChangedDispatcher))