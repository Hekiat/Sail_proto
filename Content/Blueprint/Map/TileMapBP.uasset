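; Tile map actor that spawns a grid of square or hexagon TileBP actors on BeginPlay, replacing any existing tiles.
; Positions are centred by tile type, with random height jitter and a hard-coded raised corner block.
; Tiles attach to the map and live in a flat array, indexed by square coordinates for lookup and selection-state changes.
; Tile selection is relayed through a dispatcher, and helpers convert between square and cube-style hex coordinates.
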(event Custom|Event%20Generate
  (Generation|GenerareTiles))

(event EventBeginPlay
  (CallFunction|EventGenerate))

(event Collision|EventActorBeginOverlap
  (params (OtherActor :type Actor%20Object%20Reference)))

(event EventTick
  (params (DeltaSeconds :type Float%20%28single-precision%29)))

(fn ConstructionScript)

(fn GenerareTiles
  (bind _tiles (Variables|Default|GetTiles))
  (Utilities|FlowControl|Sequence
    (:then_0
      (for _array_element _tiles
        (Actor|DestroyActor _array_element))
      (Utilities|Array|Clear _tiles))
    (:then_1
      (for _index (range 0 (- (Variables|Default|GetxTileCount) 1))
        (for _index_2 (range 0 (- (Variables|Default|GetyTileCount) 1))
          (bind _position (Generation|GenerateTilePosition (Utilities|Struct|MakeIntVector _index _index_2 0) (Variables|Default|GetTileType)))
          (bind _returnvalue (Game|SpawnActorfromClass "/Game/Blueprint/Map/TileBP.TileBP_C" (Math|Transform|MakeTransform (+ _position (Math|Vector|MakeVector 0.0 0.0 (* (Math|Random|RandomFloat) 3e+01))) "0, 0, 0" (Math|Conversions|ToVector(Float) (/ (Variables|Default|GetTileSize) 1e+02))) "Undefined" 0 (Utilities|Struct|MakeIntVector _index _index_2 0) (Variables|Default|GetTileType) self 0))
          (Transformation|AttachActorToActor _returnvalue self "None" "KeepRelative" "KeepRelative" "KeepRelative" true)
          (Utilities|Array|Add (Variables|Default|GetTiles) _returnvalue)
          (EventDispatchers|BindEventtoOnSelectedDispatcher _returnvalue (EventDispatchers|CreateEvent :!event OnTileSelected)))))))

(fn TilePosition
  (params (Coord :type Grid%20Coord%20Structure))
  (bind _ytilecount (Variables|Default|GetyTileCount))
  (bind _returnvalue (* _ytilecount (.x (.squarecoord Coord))))
  (bind _returnvalue_2 (+ _returnvalue (.y (.squarecoord Coord))))
  (if (Utilities|Array|IsValidIndex (Variables|Default|GetTiles) _returnvalue_2)
    (return (+ (Transformation|GetActorLocation (Utilities|Array|Get(acopy) (Variables|Default|GetTiles) _returnvalue_2)) (Math|Vector|MakeVector 0.0 0.0 (/ (Variables|Default|GetTileSize) 2.0))))
    (else
      (Development|PrintString "Wrong Tile Coord")
      (return "0, 0, 0"))))

(fn SetTilesSelectionStatus
  (params (Indices :type Array%20of%20Grid%20Coord%20Structures) (Mode :type TileStatusEnum%20Enum :default "NewEnumerator1"))
  (for _array_element Indices
    (bind _tile (CallFunction|GetTile _array_element))
    (Default|SetSelectionStatus _tile Mode)))

(fn ClearTilesSelectionStatus
  (for _array_element (Variables|Default|GetTiles)
    (Default|SetSelectionStatus _array_element "NewEnumerator3")))

(fn GetTile
  (params (Coord :type Grid%20Coord%20Structure))
  (bind _ytilecount (Variables|Default|GetyTileCount))
  (bind _returnvalue (* (.x (.squarecoord Coord)) _ytilecount))
  (bind _returnvalue_2 (+ (.y (.squarecoord Coord)) _returnvalue))
  (if (Utilities|Array|IsValidIndex (Variables|Default|GetTiles) _returnvalue_2)
    (return (Utilities|Array|Get(acopy) (Variables|Default|GetTiles) _returnvalue_2))
    (else
      (return 0))))

(fn OnTileSelected
  (params (SelectedTIle :type Tile%20BP%20Object%20Reference))
  (Default|CallOnTileSelectedDispatcher SelectedTIle))

(fn ResetTilesSelection
  (for _array_element (Variables|Default|GetTiles)
    (if (Utilities|Select :Index (Variables|/Game/Blueprint/Map/TileBP.TileBP_C|GetSelectionStatus _array_element) :NewEnumerator0 true :NewEnumerator4 true :NewEnumerator1 false :NewEnumerator2 false :NewEnumerator3 false)
      (Variables|/Game/Blueprint/Map/TileBP.TileBP_C|SetSelectionStatus _array_element "NewEnumerator1"))))

(fn GenerateTilePosition
  (params (Coord :type Int%20Vector%20Structure) (Type :type TileTypeEnum%20Enum :default "NewEnumerator1"))
  (bind _tilesize (Variables|Default|GetTileSize))
  (bind _tileoffset (Variables|Default|GetTileOffset))
  (bind _returnvalue (+ _tilesize _tileoffset))
  (switch Utilities|FlowControl|Switch|SwitchonTileTypeEnum Type
    (:NewEnumerator1
      (bind _output_get (LocalVariables|SetWidth (Variables|Default|GetTileSize)))
      (LocalVariables|SetHeight _output_get)
      (return (Math|Vector|MakeVector (- (* (.x Coord) _returnvalue) (/ (* (- (Variables|Default|GetxTileCount) 1) _returnvalue) 2.0)) (- (* (.y Coord) _returnvalue) (/ (* (- (Variables|Default|GetyTileCount) 1) _returnvalue) 2.0)) (select (and (<= (.x Coord) 3) (<= (.y Coord) 3)) 1.5e+02 0.0))))
    (:NewEnumerator2
      (LocalVariables|SetWidth (+ (Variables|Default|GetTileSize) (Variables|Default|GetTileOffset)))
      (LocalVariables|SetHeight (+ (* (Math|Float|Sqrt 3.0) (/ (Variables|Default|GetTileSize) 2.0)) (Variables|Default|GetTileOffset)))
      (switch int (Math|Integer|%(Integer) (.x Coord) 2)
        (:0
          (LocalVariables|SetBaseOffset 0.0))
        (:1
          (LocalVariables|SetBaseOffset (/ (LocalVariables|GetHeight) 2.0))))
      (if (and (<= (.x Coord) 3) (<= (.y Coord) 3))
        (return (+ (- (Math|Vector|MakeVector (- (* (.x Coord) (LocalVariables|GetWidth)) (* (.x Coord) (/ (LocalVariables|GetWidth) 4.0))) (+ (* (.y Coord) (LocalVariables|GetHeight)) (LocalVariables|GetBaseOffset)) 0.0) (/ (Math|Vector|MakeVector (* (* (Variables|Default|GetxTileCount) (LocalVariables|GetWidth)) 0.75) (* (Variables|Default|GetyTileCount) (LocalVariables|GetHeight)) 0.0) 2.0)) "0, 0,150.000000"))
        (else
          (return (- (Math|Vector|MakeVector (- (* (.x Coord) (LocalVariables|GetWidth)) (* (.x Coord) (/ (LocalVariables|GetWidth) 4.0))) (+ (* (.y Coord) (LocalVariables|GetHeight)) (LocalVariables|GetBaseOffset)) 0.0) (/ (Math|Vector|MakeVector (* (* (Variables|Default|GetxTileCount) (LocalVariables|GetWidth)) 0.75) (* (Variables|Default|GetyTileCount) (LocalVariables|GetHeight)) 0.0) 2.0))))))))

(fn ToHexCoord
  (params (Coord :type Int%20Vector%20Structure))
  (bind _returnvalue (Math|Integer|%(Integer) (.x Coord) 2))
  (bind _returnvalue_2 (Utilities|Select :Index _returnvalue :Option%200 0 :Option%201 1))
  (bind _returnvalue_3 (- (.x Coord) _returnvalue_2))
  (bind _returnvalue_4 (/ _returnvalue_3 2))
  (bind _returnvalue_5 (- (.y Coord) _returnvalue_4))
  (return (Utilities|Struct|MakeIntVector (.x Coord) (- (* (.x Coord) -1) _returnvalue_5) _returnvalue_5)))

(fn ToSquareCoord
  (params (HexCoord :type Int%20Vector%20Structure))
  (return (Utilities|Struct|MakeIntVector (.x HexCoord) (- (+ (.z HexCoord) 1) (/ (- (.x HexCoord) (Math|Integer|%(Integer) (.x HexCoord) 2)) 2)) 0)))