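; Level manager actor that spawns the tile map at BeginPlay, caches the player pawn and provides grid queries and pathfinding.
; GetPath runs an A*-style search with uniform step cost, returning the path ordered goal to start.
; Neighbors yields four bounds-checked adjacent tiles, plus two parity-offset ones for hexagon maps.
; The heuristic is only the cross-product deviation from the straight start-to-goal line, with no distance term.
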(event EventBeginPlay
  (Utilities|FlowControl|Sequence
    (:then_0
      (bind _asmain_character_bp (Utilities|Casting|CastToMainCharacterBP (Game|Player|GetPlayerPawn 0)))
      (Variables|Default|SetPlayerRef _asmain_character_bp))
    (:then_1
      (bind _returnvalue (Game|SpawnActorfromClass "/Game/Blueprint/Map/TileMapBP.TileMapBP_C" (Math|Transform|MakeTransform "0, 0, 0" "0, 0, 0" "1,1,1") "Undefined" 0 (Variables|Default|GetxTileCount) (Variables|Default|GetyTileCount) "NewEnumerator2" 0))
      (Variables|Default|SetTileMap _returnvalue))))

(event Collision|EventActorBeginOverlap
  (params (OtherActor :type Actor%20Object%20Reference)))

(event EventTick
  (params (DeltaSeconds :type Float%20%28single-precision%29)))

(fn ConstructionScript)

(fn TileCenterPosition
  (params (Coord :type Grid%20Coord%20Structure))
  (bind _position (Default|TilePosition (Variables|Default|GetTileMap) Coord))
  (return _position))

(fn IsCoordValid
  (params (Coordinate :type Grid%20Coord%20Structure))
  (return (and (Math|Integer|InRange(Integer) (.x (.squarecoord Coordinate)) 0 (Variables|Default|GetxTileCount) true false) (Math|Integer|InRange(Integer) (.y (.squarecoord Coordinate)) 0 (Variables|Default|GetyTileCount) true false))))

(fn GetPath
  (params (From :type Grid%20Coord%20Structure) (Goal :type Grid%20Coord%20Structure))
  (bind _priority (LocalVariables|GetPriority))
  ;[1 1 1] Initialization
  (Utilities|Array|Add (LocalVariables|GetFrontier) From)
  (Utilities|Map|Add (LocalVariables|GetPriority) From 0.0)
  (Utilities|Map|Add (LocalVariables|GetCameFrom) From From)
  (Utilities|Map|Add (LocalVariables|GetCostSoFar) From 0.0)
  (while (!= (Utilities|Array|Length (LocalVariables|GetFrontier)) 0)
    ;[1 1 1] Read Possible Best
    (bind _values (Utilities|Map|Values _priority))
    (bind _keys (Utilities|Map|Keys _priority))
    (bind _output_get (LocalVariables|SetCurrent (Utilities|Array|Get(acopy) _keys (.IndexOfMinValue (Math|Float|MinOfFloatArray _values)))))
    (Utilities|Map|Remove _priority _output_get)
    (Utilities|Array|RemoveItem (LocalVariables|GetFrontier) (LocalVariables|GetCurrent))
    ;[1 1 1] Goal Reached?
    (if (and (== (.x (.squarecoord (LocalVariables|GetCurrent))) (.x (.squarecoord Goal))) (== (.y (.squarecoord (LocalVariables|GetCurrent))) (.y (.squarecoord Goal))))
      (LocalVariables|SetCurrent Goal)
      (while (or (!= (.x (.squarecoord (LocalVariables|GetCurrent))) (.x (.squarecoord From))) (!= (.y (.squarecoord (LocalVariables|GetCurrent))) (.y (.squarecoord From))))
        (Utilities|Array|Add (LocalVariables|GetReconstructedPath) (LocalVariables|GetCurrent))
        (LocalVariables|SetCurrent (.Value (Utilities|Map|Find (LocalVariables|GetCameFrom) (LocalVariables|GetCurrent)))))
      (Utilities|Array|Add (LocalVariables|GetReconstructedPath) From)
      (return (LocalVariables|GetReconstructedPath))
      (else
        ;[1 1 1] Add Children to frontier
        (for _array_element (AStar|Neighbors (LocalVariables|GetCurrent))
          (LocalVariables|SetCurrentNeighbor _array_element)
          (LocalVariables|SetNewCost (+ (.Value (Utilities|Map|Find (LocalVariables|GetCostSoFar) (LocalVariables|GetCurrent))) (AStar|Costfromto (LocalVariables|GetCurrent) (LocalVariables|GetCurrentNeighbor))))
          (if (Utilities|Map|Contains (LocalVariables|GetCostSoFar) (LocalVariables|GetCurrentNeighbor))
            (if (< (LocalVariables|GetNewCost) (.Value (Utilities|Map|Find (LocalVariables|GetCostSoFar) (LocalVariables|GetCurrentNeighbor))))
              (Utilities|Map|Add (LocalVariables|GetCostSoFar) (LocalVariables|GetCurrentNeighbor) (LocalVariables|GetNewCost) :!label _label)
              (Utilities|Map|Add (LocalVariables|GetPriority) (LocalVariables|GetCurrentNeighbor) (+ (LocalVariables|GetNewCost) (AStar|Heuristic From (LocalVariables|GetCurrentNeighbor) Goal)))
              (Utilities|Array|Add (LocalVariables|GetFrontier) (LocalVariables|GetCurrentNeighbor))
              (Utilities|Map|Add (LocalVariables|GetCameFrom) (LocalVariables|GetCurrentNeighbor) (LocalVariables|GetCurrent)))
            (else
              (goto _label)))))))
  (return 0))

(fn Neighbors
  (params (Coord :type Grid%20Coord%20Structure))
  (bind _returnvalue (Math|Integer|%(Integer) (.x (.squarecoord Coord)) 2))
  (bind _returnvalue_2 (== _returnvalue 0))
  (bind _returnvalue_3 (select _returnvalue_2 -1 1))
  (Utilities|FlowControl|Sequence
    (:then_0
      ;[1 1 1] X-1, Y
      (LocalVariables|SetCurrentNeighbor (Class|FGridCoordLib|MakeGridCoordfromSquare (Utilities|Struct|MakeSquareCoord (- (.x (.squarecoord Coord)) 1) (.y (.squarecoord Coord)))))
      (if (CallFunction|IsCoordValid (LocalVariables|GetCurrentNeighbor)) :!label _label
        (Utilities|Array|Add (LocalVariables|GetNeighborList) (LocalVariables|GetCurrentNeighbor))))
    (:then_1
      ;[1 1 1] X, Y-1
      (LocalVariables|SetCurrentNeighbor (Class|FGridCoordLib|MakeGridCoordfromSquare (Utilities|Struct|MakeSquareCoord (.x (.squarecoord Coord)) (- (.y (.squarecoord Coord)) 1))))
      (goto _label))
    (:then_2
      ;[1 1 1] X+1, Y
      (LocalVariables|SetCurrentNeighbor (Class|FGridCoordLib|MakeGridCoordfromSquare (Utilities|Struct|MakeSquareCoord (+ (.x (.squarecoord Coord)) 1) (.y (.squarecoord Coord)))))
      (goto _label))
    (:then_3
      ;[1 1 1] X, Y+1
      (LocalVariables|SetCurrentNeighbor (Class|FGridCoordLib|MakeGridCoordfromSquare (Utilities|Struct|MakeSquareCoord (.x (.squarecoord Coord)) (+ (.y (.squarecoord Coord)) 1))))
      (goto _label))
    (:then_4
      ;[1 1 1] Hexagon only
      (if (Utilities|Enum|Equal(Enum) (Variables|/Game/Blueprint/Map/TileMapBP.TileMapBP_C|GetTileType (Variables|Default|GetTileMap)) "NewEnumerator2")
        (Utilities|FlowControl|Sequence
          (:then_0
            ;[1 1 1] Top
            (LocalVariables|SetCurrentNeighbor (Class|FGridCoordLib|MakeGridCoordfromSquare (Utilities|Struct|MakeSquareCoord (- (.x (.squarecoord Coord)) 1) (+ (.y (.squarecoord Coord)) _returnvalue_3))))
            (goto _label))
          (:then_1
            ;[1 1 1] Bottom
            (LocalVariables|SetCurrentNeighbor (Class|FGridCoordLib|MakeGridCoordfromSquare (Utilities|Struct|MakeSquareCoord (+ (.x (.squarecoord Coord)) 1) (+ _returnvalue_3 (.y (.squarecoord Coord))))))
            (goto _label)))))
    (:then_5
      (return (LocalVariables|GetNeighborList)))))

(fn Costfromto
  (params (From :type Grid%20Coord%20Structure) (To :type Grid%20Coord%20Structure))
  (return 1.0))

(fn Heuristic
  (params (Start :type Grid%20Coord%20Structure) (Current :type Grid%20Coord%20Structure) (Goal :type Grid%20Coord%20Structure))
  (return (Math|Float|Absolute(Float) (- (* (Math|Conversions|ToFloat(Integer) (- (.x (.squarecoord Current)) (.x (.squarecoord Goal)))) (Math|Conversions|ToFloat(Integer) (- (.y (.squarecoord Start)) (.y (.squarecoord Goal))))) (* (Math|Conversions|ToFloat(Integer) (- (.x (.squarecoord Start)) (.x (.squarecoord Goal)))) (Math|Conversions|ToFloat(Integer) (- (.y (.squarecoord Current)) (.y (.squarecoord Goal)))))))))