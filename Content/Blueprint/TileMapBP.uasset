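; TileMapBP is an actor that builds a centered grid of TileBP tiles and provides their world positions.
; The construction script clears the Tiles array, then spawns tiles as child actor components, spaced and scaled by tile width and offset.
; Each tile stores its grid indices and joins the flat, column-ordered array.
; TilePosition maps a coordinate to that array and returns a point half a tile width above the tile's cube, printing an error when invalid.
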(event EventBeginPlay)

(event Collision|EventActorBeginOverlap
  (params (OtherActor :type Actor%20Object%20Reference)))

(event EventTick
  (params (DeltaSeconds :type Float%20%28single-precision%29)))

(fn ConstructionScript
  (CallFunction|GenerareTiles))

(fn GenerareTiles
  (bind _tileoffset (Variables|Default|GetTileOffset))
  (bind _tilewidth (Variables|Default|GetTileWidth))
  (bind _returnvalue (+ _tilewidth _tileoffset))
  (Utilities|FlowControl|Sequence
    (:then_0
      (Utilities|Array|Clear (Variables|Default|GetTiles)))
    (:then_1
      (for _index (range 0 (- (Variables|Default|GetxTileCount) 1))
        (for _index_2 (range 0 (- (Variables|Default|GetyTileCount) 1))
          (bind _returnvalue_2 (AddComponent|AddChildActorComponent false (Math|Transform|MakeTransform (Math|Vector|MakeVector (- (* _index _returnvalue) (/ (* (- (Variables|Default|GetxTileCount) 1) _returnvalue) 2.0)) (- (* _index_2 _returnvalue) (/ (* (- (Variables|Default|GetyTileCount) 1) _returnvalue) 2.0)) 0.0) "0, 0, 0" (Math|Conversions|ToVector(Float) (/ (Variables|Default|GetTileWidth) 1e+02)))))
          (ChildActorComponent|SetChildActorClass _returnvalue_2 "/Game/Blueprint/TileBP.TileBP_C")
          (bind _astile_bp (Utilities|Casting|CastToTileBP (Variables|/Script/Engine.ChildActorComponent|GetChildActor _returnvalue_2)))
          (Variables|/Game/Blueprint/TileBP.TileBP_C|SetvIndex _astile_bp _index_2)
          (Variables|/Game/Blueprint/TileBP.TileBP_C|SethIndex _astile_bp _index)
          (Utilities|Array|Add (Variables|Default|GetTiles) _astile_bp))))))

(fn TilePosition
  (params (Coord :type Int%20Point%20Structure))
  (bind _ytilecount (Variables|Default|GetyTileCount))
  (bind _returnvalue (* _ytilecount (.x Coord)))
  (bind _returnvalue_2 (+ _returnvalue (.y Coord)))
  (if (Utilities|Array|IsValidIndex (Variables|Default|GetTiles) _returnvalue_2)
    (return (+ (Transformation|GetWorldLocation (Variables|/Game/Blueprint/TileBP.TileBP_C|GetCube (Utilities|Array|Get(acopy) (Variables|Default|GetTiles) _returnvalue_2))) (Math|Vector|MakeVector 0.0 0.0 (/ (Variables|Default|GetTileWidth) 2.0))))
    (else
      (Development|PrintString "Wrong Tile Coord")
      (return "0, 0, 0"))))