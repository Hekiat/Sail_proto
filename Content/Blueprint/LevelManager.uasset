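; LevelManager is an actor that sets up the tile-based level and answers grid queries.
; On BeginPlay it caches the player's MainCharacterBP and spawns a TileMapBP sized by its X and Y tile counts, keeping a reference to it.
; TileCenterPosition asks the tile map for a coordinate's position, and IsCoordValid checks that a coordinate lies within the grid bounds.
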(event EventBeginPlay
  (Utilities|FlowControl|Sequence
    (:then_0
      (bind _asmain_character_bp (Utilities|Casting|CastToMainCharacterBP (Game|Player|GetPlayerPawn 0)))
      (Variables|Default|SetPlayerRef _asmain_character_bp))
    (:then_1
      (bind _returnvalue (Game|SpawnActorfromClass "/Game/Blueprint/TileMapBP.TileMapBP_C" (Math|Transform|MakeTransform "0, 0, 0" "0, 0, 0" "1,1,1") "Undefined" 0 (Variables|Default|GetxTileCount) (Variables|Default|GetyTileCount) 0))
      (Variables|Default|SetTileMap _returnvalue))))

(event Collision|EventActorBeginOverlap
  (params (OtherActor :type Actor%20Object%20Reference)))

(event EventTick
  (params (DeltaSeconds :type Float%20%28single-precision%29)))

(fn ConstructionScript)

(fn TileCenterPosition
  (params (Coord :type Int%20Vector%20Structure))
  (bind _position (Default|TilePosition (Variables|Default|GetTileMap) Coord))
  (return _position))

(fn IsCoordValid
  (params (Coord :type Int%20Vector%20Structure))
  (return (Math|Boolean|ANDBoolean (>= (.x Coord) 0) (>= (.y Coord) 0) (< (.x Coord) (Variables|Default|GetxTileCount)) (< (.y Coord) (Variables|Default|GetyTileCount)))))