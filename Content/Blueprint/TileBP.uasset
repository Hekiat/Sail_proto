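; TileBP is a grid tile that can be selected by clicking a widget shown on it.
; On BeginPlay it starts non-selectable and passes its coordinate, self reference and click handler to the ControllerTileWidget inside SelectionWidget.
; Left mouse input is forwarded through a widget interaction component, and a click fires the tile's selected dispatcher.
; SetSelectable stores the selection status and shows the widget for every state except NotSelectable.
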(event Custom|OnTileClicked
  (Default|CallOnSelectedDispatcher self))

(event EventBeginPlay
  (VariableGetSet|SetSelectable "NewEnumerator3")
  (bind _ascontroller_tile_widget (Utilities|Casting|CastToControllerTileWidget (UserInterface|GetUserWidgetObject (Variables|Components|GetSelectionWidget))))
  (Variables|/Game/UI/Controller/ControllerTileWidget.ControllerTileWidget_C|SetPosition _ascontroller_tile_widget (Variables|Default|GetCoord))
  (Variables|/Game/UI/Controller/ControllerTileWidget.ControllerTileWidget_C|SetTileRef _ascontroller_tile_widget self)
  (EventDispatchers|AssignOnClicked _ascontroller_tile_widget (delegate Custom|OnTileClicked)))

(event Collision|EventActorBeginOverlap
  (params (OtherActor :type Actor%20Object%20Reference)))

(event EventTick
  (params (DeltaSeconds :type Float%20%28single-precision%29)))

(event Input|MouseEvents|LeftMouseButton
  (params (Key :type Key%20Structure))
  (bind _selectionwidgetinteraction (Variables|Components|GetSelectionWidgetInteraction))
  (:Pressed
    (Class|WidgetInteractionComponent|PressPointerKey _selectionwidgetinteraction Key))
  (:Released
    (Class|WidgetInteractionComponent|ReleasePointerKey _selectionwidgetinteraction Key)))

(fn ConstructionScript)

(fn SetSelectable
  (params (SelectionType :type TileSelectionEnum%20Enum :default "NewEnumerator3"))
  (bind _output_get (Variables|Default|SetSelectionStatus SelectionType))
  (Rendering|SetVisibility (Variables|Components|GetSelectionWidget) (Utilities|Select :Index _output_get :NewEnumerator0 true :NewEnumerator1 true :NewEnumerator2 true :NewEnumerator3 false) false))