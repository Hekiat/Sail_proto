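; Thread Blueprint that queues the player's function actions within a limited time-slot budget and plays them in order, clearing the queue at end of turn.
; Each registered function starts from the previous one's post-action position, or the player's grid position if first, and UpdateInitialPositions recomputes that chain.
; Playback is event-driven: each function's OnPlayEnded dispatcher triggers the next, and the thread broadcasts its own OnPlayEnded after the last.
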(event Custom|Event%20End%20Turn
  (Utilities|Array|Clear (Variables|Default|GetRegisteredFunctions)))

(event EventBeginPlay)

(event Collision|EventActorBeginOverlap
  (params (OtherActor :type Actor%20Object%20Reference)))

(event EventTick
  (params (DeltaSeconds :type Float%20%28single-precision%29)))

(fn ConstructionScript)

(fn RegisterFunction
  (params (Function :type Function%20Base%20BP%20Object%20Reference))
  (bind _registeredfunctions (Variables|Default|GetRegisteredFunctions))
  (bind _returnvalue (Utilities|Array|LastIndex _registeredfunctions))
  (if (!= _returnvalue -1)
    (LocalVariables|SetInitialPosition (Default|GetPostActionPosition (Utilities|Array|Get(acopy) _registeredfunctions _returnvalue)))
    (else
      (LocalVariables|SetInitialPosition (Variables|/Game/Blueprint/MainCharacterBP.MainCharacterBP_C|GetGridPosition (Variables|Default|GetPlayerRef)))))
  (Default|Initialize Function (LocalVariables|GetInitialPosition))
  (Utilities|Array|Add (Variables|Default|GetRegisteredFunctions) Function)
  (Variables|/Game/Blueprint/FunctionActors/FunctionBaseBP.FunctionBaseBP_C|SetIsUsed Function true)
  (Default|CallOnStatusChanged Function)
  (EventDispatchers|BindEventtoOnPostActionPositionChanged Function (EventDispatchers|CreateEvent :!event UpdateInitialPositions))
  (return))

(fn AvailableTimeSlot
  (for _array_element (Variables|Default|GetRegisteredFunctions)
    (LocalVariables|SetSlotCount (+ (Utilities|Struct|BreakFunctionDataStruct (Variables|/Game/Blueprint/FunctionActors/FunctionBaseBP.FunctionBaseBP_C|GetFunctionData _array_element)) (LocalVariables|GetSlotCount))))
  (return (- (Variables|Default|GetMaxTimeSlot) (LocalVariables|GetSlotCount))))

(fn UnregisterFunction
  (params (Function :type Function%20Base%20BP%20Object%20Reference))
  (Utilities|Array|RemoveItem (Variables|Default|GetRegisteredFunctions) Function)
  (Variables|/Game/Blueprint/FunctionActors/FunctionBaseBP.FunctionBaseBP_C|SetIsUsed Function false)
  (return))

(fn IsFunctionUsable
  (params (Function :type Function%20Base%20BP%20Object%20Reference))
  (return (<= (Utilities|Struct|BreakFunctionDataStruct (Variables|/Game/Blueprint/FunctionActors/FunctionBaseBP.FunctionBaseBP_C|GetFunctionData Function)) (Helpers|AvailableTimeSlot))))

(fn UpdateInitialPositions
  (LocalVariables|SetCurrentPosition (Variables|/Game/Blueprint/MainCharacterBP.MainCharacterBP_C|GetGridPosition (Variables|Default|GetPlayerRef)))
  (for _array_element (Variables|Default|GetRegisteredFunctions)
    (Default|SetInitialPosition _array_element (LocalVariables|GetCurrentPosition))
    (LocalVariables|SetCurrentPosition (Default|GetPostActionPosition _array_element))))

(fn StartPlay
  (if (== (Utilities|Array|Length (Variables|Default|GetRegisteredFunctions)) 0)
    (Default|CallOnPlayEnded)
    (else
      (Variables|Play|SetIsPlaying true)
      (PlayFlow|PlayFunction))))

(fn OnFunctionPlayEnded
  (EventDispatchers|UnbindallEventsfromOnPlayEnded (Utilities|Array|Get(acopy) (Variables|Default|GetRegisteredFunctions) (Variables|Default|GetPlayingFunctionID)))
  (if (== (Variables|Default|GetPlayingFunctionID) (Utilities|Array|LastIndex (Variables|Default|GetRegisteredFunctions)))
    ;[1 1 1] Last Function, end of the thread play
    (Variables|Play|SetIsPlaying false)
    (Variables|Default|SetPlayingFunctionID -1)
    (Default|CallOnPlayEnded)
    (else
      ;[1 1 1] Play Next Function
      (bind _result (Math|Integer|IncrementInt (Variables|Default|GetPlayingFunctionID))
        (:%20%20
          (PlayFlow|PlayFunction _result)
          (Development|PrintString "Play Next Function"))))))

(fn PlayFunction
  (params (FunctionID :type Integer))
  (bind _output_get (Variables|Default|SetPlayingFunctionID FunctionID))
  (EventDispatchers|BindEventtoOnPlayEnded (Utilities|Array|Get(acopy) (Variables|Default|GetRegisteredFunctions) _output_get) (EventDispatchers|CreateEvent :!event OnFunctionPlayEnded))
  (Default|ActionBeginPlay (Utilities|Array|Get(acopy) (Variables|Default|GetRegisteredFunctions) _output_get)))