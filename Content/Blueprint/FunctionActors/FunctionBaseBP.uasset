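; Base actor for a turn-based "function" action with plugin slots, a cooldown and overridable play logic.
; Plugins register into fixed slots, replacing any occupant and updating its used state.
; Selection and initial position pass through a Controller, with Initialize also setting a MoveController target.
; Tick calls the stub Play while playing, EndTurn updates cooldown and clears selection, and status changes are broadcast.
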(event Custom|Event%20End%20Turn
  (if (Variables|Runtime|GetIsUsed)
    (Variables|Runtime|SetCooldownTurn (Utilities|Struct|BreakFunctionDataStruct (Variables|Default|GetFunctionData)))
    (else
      (Variables|Runtime|SetCooldownTurn (Math|Integer|Max(Integer) (- (Variables|Runtime|GetCooldownTurn) 1)))))
  (Variables|Runtime|SetIsUsed false)
  (CallFunction|SetSelected false)
  (Default|CallOnStatusChanged))

(event EventBeginPlay
  (Utilities|Array|Resize (Variables|Plugin|GetPlugins) (Variables|Plugin|GetPluginMax)))

(event EventTick
  (params (DeltaSeconds :type Float%20%28single-precision%29))
  (if (Variables|PlayFlow|GetIsPlaying)
    (PlayFlow|Play)))

(fn ConstructionScript)

(fn RegisterPlugin
  (params (Plugin :type Function%20Base%20BP%20Object%20Reference) (PluginSlotIndex :type Integer))
  (Utilities|IsValid (Utilities|Array|Get(acopy) (Variables|Plugin|GetPlugins) PluginSlotIndex)
    (:Is%20Valid
      ;[1 1 1] Remove Old
      (Plugin|UnregisterPlugin PluginSlotIndex))
    (:Is%20Not%20Valid
      _))
  ;[1 1 1] Add New
  (Utilities|Array|SetArrayElem (Variables|Plugin|GetPlugins) PluginSlotIndex Plugin)
  (Variables|FunctionBaseBP_C|SetIsUsed Plugin true)
  (Default|CallOnStatusChanged Plugin)
  (return))

(fn UnregisterPlugin
  (params (PluginSlotIndex :type Integer))
  (bind _plugins (Variables|Plugin|GetPlugins))
  (bind _output (Utilities|Array|Get(acopy) _plugins PluginSlotIndex))
  (Variables|FunctionBaseBP_C|SetIsUsed _output false)
  (Default|CallOnStatusChanged _output)
  (Utilities|Array|SetArrayElem (Variables|Plugin|GetPlugins) PluginSlotIndex 0)
  ;[1 0 0.04851] Debug Print
  (Development|PrintString (Utilities|String|Append "Slot " (Utilities|String|ToString(Integer) PluginSlotIndex) " Unregistered from " (Utilities|GetDisplayName self))))

(fn IsPluginUsable
  (params (Plugin :type Function%20Base%20BP%20Object%20Reference))
  (return true))

(fn SetSelected
  (params (Selected :type Boolean))
  (bind _controller (Variables|Default|GetController))
  (Utilities|IsValid _controller
    (:Is%20Valid
      (Default|SetActive _controller Selected))))

(fn SetInitialPosition
  (params (Coord :type Int%20Vector%20Structure))
  (Utilities|IsValid (Variables|Default|GetController)
    (:Is%20Valid
      (bind _output_get (Variables|Runtime|SetInitial%20Position Coord))
      (Default|SetInitialPosition (Variables|Default|GetController) _output_get))))

(fn GetPostActionPosition
  (return (Variables|Runtime|GetInitial%20Position)))

(fn Initialize
  (params (Coord :type Int%20Vector%20Structure))
  (bind _controller (Variables|Default|GetController))
  (CallFunction|SetInitialPosition Coord)
  (Utilities|IsValid _controller
    (:Is%20Valid
      (bind _asmove_controller (Utilities|Casting|CastToMoveController _controller))
      (Default|SetTarget _asmove_controller Coord))))

(fn Play
  (Development|PrintString "Base Function Play"))

(fn BeginPlay
  (Variables|PlayFlow|SetIsPlaying true)
  (Default|CallOnStatusChanged))

(fn EndPlay
  (Variables|PlayFlow|SetIsPlaying false)
  (Default|CallOnStatusChanged)
  (Default|CallOnPlayEnded))