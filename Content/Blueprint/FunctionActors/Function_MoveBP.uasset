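; Move action for a tile-based game that lets the player pick a destination and walks the main character to it.
; Spawns a radial MoveController at BeginPlay and relays its target changes as post-action position changes.
; While the controller is active, Tick highlights the path from the initial position to the hovered tile.
; ActionPlay issues MoveToCoord toward the first target, ending the action once the pawn is near the tile center.
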(event Custom|OnPostActionPositionChanged_Event
  (Default|CallOnPostActionPositionChanged))

(event EventBeginPlay
  (bind _returnvalue (Game|SpawnActorfromClass :Class "/Game/Blueprint/Controller/MoveController.MoveController_C" :CollisionHandlingOverride "Undefined" :Radial true :PlayerRef (Variables|Default|GetPlayerRef) :Instigator 0))
  (bind _output_get (Variables|Default|SetController _returnvalue))
  (bind _asmove_controller (Utilities|Casting|CastToMoveController _output_get))
  (Default|SetActive _asmove_controller false)
  (EventDispatchers|BindEventtoOnTargetChanged _asmove_controller (delegate Custom|OnPostActionPositionChanged_Event)))

(event Collision|EventActorBeginOverlap
  (params (OtherActor :type Actor%20Object%20Reference)))

(event EventTick
  (params (DeltaSeconds :type Float%20%28single-precision%29))
  (bind _playerref (Variables|Default|GetPlayerRef))
  (bind _levelmanager (Variables|/Game/Blueprint/MainCharacterBP.MainCharacterBP_C|GetLevelManager _playerref))
  (bind _tilemap (Variables|/Game/Blueprint/Map/LevelManager.LevelManager_C|GetTileMap _levelmanager))
  (|CallParentFunction 0.0)
  (if (Variables|/Game/Blueprint/Controller/ControllerBase.ControllerBase_C|GetIsActive (Variables|Default|GetController))
    (Default|ResetTilesSelection _tilemap)
    (for _array_element (Variables|/Game/Blueprint/Map/TileMapBP.TileMapBP_C|GetTiles _tilemap)
      (bind _ascontroller_tile_widget (Utilities|Casting|CastToControllerTileWidget (UserInterface|GetUserWidgetObject (Variables|/Game/Blueprint/Map/TileBP.TileBP_C|GetSelectionWidget _array_element))))
      (Utilities|IsValid (Variables|/Game/UI/Controller/ControllerTileWidget.ControllerTileWidget_C|GetNeutralWidget _ascontroller_tile_widget)
        (:Is%20Valid
          (if (Widget|IsHovered (Variables|/Game/UI/Controller/ControllerTileWidget.ControllerTileWidget_C|GetNeutralWidget _ascontroller_tile_widget))
            (bind _path (Default|GetPath _levelmanager (Variables|Default|GetInitial%20Position) (Variables|/Game/Blueprint/Map/TileBP.TileBP_C|GetCoord _array_element)))
            (for (_array_element_2 _array_index) _path
              (if (not (== _array_index 0))
                (bind _tile (Default|GetTile (Variables|/Game/Blueprint/Map/LevelManager.LevelManager_C|GetTileMap _levelmanager) _array_element_2))
                (Default|SetSelectionStatus _tile "NewEnumerator4")))))))))

(event EventActionPlay
  (if (< (Math|Vector|VectorLengthXY (- (Default|TileCenterPosition (Variables|/Game/Blueprint/Framework/MainGameMode.MainGameMode_C|GetLevelManager (.AsMain%20Game%20Mode (Utilities|Casting|CastToMainGameMode (Game|GetGameMode)))) (Utilities|Array|Get(acopy) (Variables|/Game/Blueprint/Controller/ControllerBase.ControllerBase_C|GetTargets (Variables|Default|GetController)))) (Transformation|GetActorLocation (Game|Player|GetPlayerPawn 0)))) 1e+01)
    (Development|PrintString "Target Reached")
    (CallFunction|ActionEndPlay)
    (else
      (Default|MovetoCoord (.AsMain%20Character%20BP (Utilities|Casting|CastToMainCharacterBP (Game|Player|GetPlayerPawn 0))) (Utilities|Array|Get(acopy) (Variables|/Game/Blueprint/Controller/ControllerBase.ControllerBase_C|GetTargets (Variables|Default|GetController)))))))

(fn ConstructionScript
  (|CallParentFunction))

(fn GetPostActionPosition
  (return (Utilities|Array|Get(acopy) (Variables|/Game/Blueprint/Controller/ControllerBase.ControllerBase_C|GetTargets (Variables|Default|GetController)))))