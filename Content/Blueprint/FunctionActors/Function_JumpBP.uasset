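; Jump action actor that moves the player in an arc to a targeted tile.
; On BeginPlay it spawns a MoveController with range 2, whose first target becomes the landing tile.
; When the action begins it disables capsule gravity and physics collision, then a duration-scaled timeline lerps tile centers, adds a height curve and turns the mesh.
; On finish it ends the action and restores collision, leaving gravity off.
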(event Custom|MovementModeChangedDelegate_Event_0
  (params (Character :type Character%20Object%20Reference) (PrevMovementMode :type EMovementMode%20Enum :default "MOVE_None") (PreviousCustomMode :type Byte))
  (Development|PrintString "End jump"))

(event EventBeginPlay
  (|CallParentFunction)
  (bind _returnvalue (Game|SpawnActorfromClass :Class "/Game/Blueprint/Controller/MoveController.MoveController_C" :CollisionHandlingOverride "Undefined" :Range 2 :PlayerRef (Variables|Default|GetPlayerRef) :Instigator 0))
  (Variables|Default|SetController _returnvalue))

(event Collision|EventActorBeginOverlap
  (params (OtherActor :type Actor%20Object%20Reference)))

(event EventTick
  (params (DeltaSeconds :type Float%20%28single-precision%29))
  (|CallParentFunction DeltaSeconds) ; This node is disabled and will not be called.\nDrag off pins to build functionality.
)

(event EventActionBeginPlay
  (bind _playerref (Variables|Default|GetPlayerRef))
  (bind _playerref_2 (Variables|Default|GetPlayerRef))
  (bind _playerref_3 (Variables|Default|GetPlayerRef))
  (bind _levelmanager (Variables|/Game/Blueprint/MainCharacterBP.MainCharacterBP_C|GetLevelManager _playerref_2))
  (bind _mesh (Variables|/Script/Engine.Character|GetMesh _playerref))
  (bind _capsulecomponent (Variables|/Script/Engine.Character|GetCapsuleComponent _playerref_3))
  (|CallParentFunction)
  (Physics|SetEnableGravity _capsulecomponent false)
  (Collision|SetCollisionEnabled _capsulecomponent "QueryOnly")
  (Variables|Default|SetJumpEndPos (Default|TileCenterPosition _levelmanager (Utilities|Array|Get(acopy) (Variables|/Game/Blueprint/Controller/ControllerBase.ControllerBase_C|GetTargets (Variables|Default|GetController)))))
  (Variables|Default|SetJumpStartPos (Default|TileCenterPosition _levelmanager (Variables|Default|GetInitial%20Position)))
  (Components|Timeline|SetPlayRate (Variables|Default|GetJumpTimeline) (/ 1.0 (Variables|Default|GetJumpDuration)))
  (bind (_direction _position _jumpheight) (Timeline|JumpTimeline PlayFromStart)
    (:Update
      (Transformation|SetActorLocation (Variables|Default|GetPlayerRef) (+ (Math|Vector|Lerp(Vector) (Variables|Default|GetJumpStartPos) (Variables|Default|GetJumpEndPos) _position) (Math|Vector|MakeVector 0.0 0.0 (Components|Capsule|GetScaledCapsuleHalfHeight (Variables|/Script/Engine.Character|GetCapsuleComponent (Variables|Default|GetPlayerRef)))) (* (Math|Vector|MakeVector 0.0 0.0 (Variables|Default|GetJumpHeight)) _jumpheight)) false false)
      (Transformation|SetWorldRotation _mesh (Math|Rotator|Lerp(Rotator) (Transformation|GetWorldRotation _mesh) (.rotation (Class|KismetAnimationLibrary|Lookat (Math|Transform|MakeTransform (Variables|Default|GetJumpStartPos) "0, 0, 0" "1,1,1") (Variables|Default|GetJumpEndPos) "0.000000,1.000000,0.000000" true "0,0.000000,1.000000" 0.0)) _position true) false false))
    (:Finished
      (CallFunction|ActionEndPlay)
      (Collision|SetCollisionEnabled (Variables|/Script/Engine.Character|GetCapsuleComponent (Variables|Default|GetPlayerRef)) "QueryAndPhysics"))))

(event EventActionPlay
  (bind _playerref (Variables|Default|GetPlayerRef))
  (bind _mesh (Variables|/Script/Engine.Character|GetMesh _playerref))
  (bind (_direction _position _jumpheight) (Timeline|JumpTimeline Play)
    (:Update
      (Transformation|SetActorLocation (Variables|Default|GetPlayerRef) (+ (Math|Vector|Lerp(Vector) (Variables|Default|GetJumpStartPos) (Variables|Default|GetJumpEndPos) _position) (Math|Vector|MakeVector 0.0 0.0 (Components|Capsule|GetScaledCapsuleHalfHeight (Variables|/Script/Engine.Character|GetCapsuleComponent (Variables|Default|GetPlayerRef)))) (* (Math|Vector|MakeVector 0.0 0.0 (Variables|Default|GetJumpHeight)) _jumpheight)) false false)
      (Transformation|SetWorldRotation _mesh (Math|Rotator|Lerp(Rotator) (Transformation|GetWorldRotation _mesh) (.rotation (Class|KismetAnimationLibrary|Lookat (Math|Transform|MakeTransform (Variables|Default|GetJumpStartPos) "0, 0, 0" "1,1,1") (Variables|Default|GetJumpEndPos) "0.000000,1.000000,0.000000" true "0,0.000000,1.000000" 0.0)) _position true) false false))
    (:Finished
      (CallFunction|ActionEndPlay)
      (Collision|SetCollisionEnabled (Variables|/Script/Engine.Character|GetCapsuleComponent (Variables|Default|GetPlayerRef)) "QueryAndPhysics"))))

(fn ConstructionScript
  (|CallParentFunction))