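; ControllerBase is a base actor for controllers that sit on a tile map and can react to tile selection while active.
; On BeginPlay it caches the player and LevelManager, then teleports to just above the center of its initial tile.
; SetActive binds or unbinds the tile map's selection dispatcher and refreshes the widget when the state changes.
; UpdateWidget and OnSelectedTileChanged are empty stubs here.
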(event EventBeginPlay
  (CallFunction|Initialize))

(event Collision|EventActorBeginOverlap
  (params (OtherActor :type Actor%20Object%20Reference)))

(event EventTick
  (params (DeltaSeconds :type Float%20%28single-precision%29)))

(fn ConstructionScript)

(fn SetInitialPosition
  (params (Origin :type Int%20Vector%20Structure))
  (bind _output_get (Variables|Common|SetInitialPosition Origin))
  (bind _position (Default|TileCenterPosition (Variables|Common|GetLevelManagerRef) _output_get))
  (Transformation|SetActorLocation (+ _position "0, 0,5.000000") false true)
  (Common|UpdateWidget))

(fn UpdateWidget
  (return false))

(fn Initialize
  (bind _asmain_character_bp (Utilities|Casting|CastToMainCharacterBP (Game|Player|GetPlayerPawn 0)))
  (Variables|Common|SetPlayerRef _asmain_character_bp)
  (bind _outactors (Actor|GetAllActorsOfClass "/Game/Blueprint/LevelManager.LevelManager_C"))
  (Variables|Common|SetLevelManagerRef (Utilities|Array|Get(acopy) _outactors))
  (CallFunction|SetInitialPosition (Variables|Common|GetInitialPosition)))

(fn SetActive
  (params (Active :type Boolean))
  (bind _levelmanagerref (Variables|Common|GetLevelManagerRef))
  (bind _tilemap (Variables|/Game/Blueprint/LevelManager.LevelManager_C|GetTileMap _levelmanagerref))
  (if (Math|Boolean|NotEqual(Boolean) Active (Variables|Common|GetIsActive))
    (bind _output_get (Variables|Common|SetIsActive Active))
    (Common|UpdateWidget)
    (if _output_get
      (EventDispatchers|BindEventtoOnTileSelectedDispatcher _tilemap (EventDispatchers|CreateEvent :!event OnSelectedTileChanged))
      (else
        (EventDispatchers|UnbindEventfromOnTileSelectedDispatcher _tilemap (EventDispatchers|CreateEvent :!event OnSelectedTileChanged))))))

(fn OnSelectedTileChanged
  (params (SelectedTile :type Tile%20BP%20Object%20Reference))
  (return))