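; Grid move controller that lets the player pick a target tile within Range of an origin tile.
; On first tick it finds the LevelManager and snaps to the origin; while active, it marks valid tiles in a radial (Manhattan) or cross pattern as selectable on the TileMap.
; Activation binds tile selection events, which set the target, place a hologram there oriented from the player's position, and broadcast the change.
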(event EventBeginPlay
  (bind _asmain_character_bp (Utilities|Casting|CastToMainCharacterBP (Game|Player|GetPlayerPawn 0)))
  (Variables|Public|SetPlayerRef _asmain_character_bp))

(event Collision|EventActorBeginOverlap
  (params (OtherActor :type Actor%20Object%20Reference)))

(event EventTick
  (params (DeltaSeconds :type Float%20%28single-precision%29))
  (Utilities|FlowControl|Sequence
    (:then_0
      (Utilities|FlowControl|DoOnce false
        (:Completed
          (bind _outactors (Actor|GetAllActorsOfClass "/Game/Blueprint/LevelManager.LevelManager_C"))
          (Variables|Private|SetLevelManagerBP (Utilities|Array|Get(acopy) _outactors))
          (CallFunction|SetInitialPosition (Variables|Default|GetInitialPosition)))))
    (:then_1
      (CallFunction|SetActive (Variables|Default|GetIsActive)))))

(fn ConstructionScript)

(fn SetTarget
  (params (Position :type Int%20Vector%20Structure))
  (bind _levelmanagerbp (Variables|Private|GetLevelManagerBP))
  (bind _hologramtarget (Variables|Default|GetHologramTarget))
  (Variables|Default|SetIsTargetSet (Default|IsCoordValid _levelmanagerbp Position))
  (bind _output_get (Variables|Default|SetTarget Position))
  (bind _position (Default|TileCenterPosition _levelmanagerbp _output_get))
  (Transformation|SetWorldLocation _hologramtarget _position false true)
  (Transformation|SetWorldRotation _hologramtarget (.rotation (Class|KismetAnimationLibrary|Lookat (Math|Transform|MakeTransform (Transformation|GetActorLocation (Variables|Public|GetPlayerRef)) "0, 0, 0" "1,1,1") _position "0.000000,1.000000,0.000000" true "0,0.000000,1.000000" 0.0)) false false)
  (Rendering|SetVisibility _hologramtarget true false)
  (Default|CallOnTargetChanged))

(fn OnSelectedTileChanged
  (params (SelectedTile :type Tile%20BP%20Object%20Reference))
  (CallFunction|SetTarget (Variables|/Game/Blueprint/TileBP.TileBP_C|GetCoord SelectedTile)))

(fn WidgetLocaltoWorldCoord
  (params (LocalCoord :type Int%20Vector%20Structure))
  (bind _initialposition (Variables|Default|GetInitialPosition))
  (bind _range (Variables|Default|GetRange))
  (return (Utilities|Struct|MakeIntVector (+ (- (.x LocalCoord) _range) (.x _initialposition)) (+ (.y _initialposition) (- (.y LocalCoord) _range)) 0)))

(fn WorldtoWidgetLocalCoord
  (params (WorldCoord :type Int%20Point%20Structure))
  (bind _initialposition (Variables|Default|GetInitialPosition))
  (bind _range (Variables|Default|GetRange))
  (return (Utilities|Struct|MakeIntPoint (+ (- (.x WorldCoord) (.x _initialposition)) _range) (+ _range (- (.y WorldCoord) (.y _initialposition))))))

(fn SetInitialPosition
  (params (Origin :type Int%20Vector%20Structure))
  (bind _output_get (Variables|Default|SetInitialPosition Origin))
  (bind _position (Default|TileCenterPosition (Variables|Private|GetLevelManagerBP) _output_get))
  (Transformation|SetActorLocation (+ _position "0, 0,5.000000") false true)
  (CallFunction|UpdateWidget))

(fn UpdateWidget
  (bind _initialposition (Variables|Default|GetInitialPosition))
  (bind _range (Variables|Default|GetRange))
  (bind _initialposition_2 (Variables|Default|GetInitialPosition))
  (bind _initialposition_3 (Variables|Default|GetInitialPosition))
  (if (Variables|Default|GetIsActive)
    (Utilities|FlowControl|Sequence
      (:then_0
        (bind _index (Utilities|FlowControl|ForLoopwithBreak (- (.x _initialposition) _range) (+ (.x _initialposition) _range))
          (:LoopBody
            (bind _index_2 (Utilities|FlowControl|ForLoopwithBreak (- (.y _initialposition) _range) (+ (.y _initialposition) _range))
              (:LoopBody
                (if (and (Default|IsCoordValid (Variables|Private|GetLevelManagerBP) (Utilities|Struct|MakeIntVector _index _index_2)) (select (Variables|Default|GetRadial) (<= (+ (Math|Integer|Absolute(Integer) (- (.x _initialposition_2) _index)) (Math|Integer|Absolute(Integer) (- (.y _initialposition_2) _index_2))) (Variables|Default|GetRange)) (or (== _index_2 (.y _initialposition_3)) (== (.x _initialposition_3) _index))))
                  (Utilities|Array|Add (LocalVariables|GetenableCoord) (Utilities|Struct|MakeIntVector _index _index_2))))))))
      (:then_1
        (Default|SetTilesSelectable (Variables|/Game/Blueprint/LevelManager.LevelManager_C|GetTileMap (Variables|Private|GetLevelManagerBP)) (LocalVariables|GetenableCoord))))))

(fn SetActive
  (params (Active :type Boolean))
  (bind _levelmanagerbp (Variables|Private|GetLevelManagerBP))
  (bind _tilemap (Variables|/Game/Blueprint/LevelManager.LevelManager_C|GetTileMap _levelmanagerbp))
  (if (Math|Boolean|NotEqual(Boolean) Active (Variables|Default|GetIsActive))
    (bind _output_get (Variables|Default|SetIsActive Active))
    (CallFunction|UpdateWidget)
    (if _output_get
      (EventDispatchers|BindEventtoOnTileSelectedDispatcher _tilemap (EventDispatchers|CreateEvent :!event OnSelectedTileChanged))
      (else
        (EventDispatchers|UnbindEventfromOnTileSelectedDispatcher _tilemap (EventDispatchers|CreateEvent :!event OnSelectedTileChanged))))))