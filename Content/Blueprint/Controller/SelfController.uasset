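; SelfController is a child controller Blueprint that limits tile selection to the player's own tile, apparently for self-targeted choices.
; Its updateWidget override runs the parent logic, clears selectable tiles on the level manager's TileMap, then marks only the player's grid position selectable and returns false.
; The event graph holds only disabled default events, and the construction script just calls its parent.
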(event EventBeginPlay
  (|CallParentFunction) ; This node is disabled and will not be called.\nDrag off pins to build functionality.
)

(event Collision|EventActorBeginOverlap
  (params (OtherActor :type Actor%20Object%20Reference))
  (|CallParentFunction OtherActor) ; This node is disabled and will not be called.\nDrag off pins to build functionality.
)

(event EventTick
  (params (DeltaSeconds :type Float%20%28single-precision%29))
  (|CallParentFunction DeltaSeconds) ; This node is disabled and will not be called.\nDrag off pins to build functionality.
)

(fn ConstructionScript
  (|CallParentFunction))

(fn UpdateWidget
  (bind _levelmanagerref (Variables|Default|GetLevelManagerRef))
  (bind _tilemap (Variables|/Game/Blueprint/LevelManager.LevelManager_C|GetTileMap _levelmanagerref))
  (|CallParentFunction)
  (Default|ClearTilesSelectable _tilemap)
  (Default|SetTilesSelectable _tilemap (Utilities|Array|MakeArray (Variables|/Game/Blueprint/MainCharacterBP.MainCharacterBP_C|GetGridPosition (Variables|Default|GetPlayerRef))))
  (return false))