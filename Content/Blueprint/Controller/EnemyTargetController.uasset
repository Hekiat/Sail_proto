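; Targeting controller that makes the tiles occupied by enemies selectable on the level's tile map.
; When active, its widget update adds every EnemyBaseBP position to ValidCoord, resets selectable tiles, applies that list and separately sets the origin tile's selectable state.
; When inactive, the update clears selectable tiles.
; A selected-tile change only draws a temporary debug sphere at that tile's center.
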(event EventBeginPlay
  (|CallParentFunction))

(event Collision|EventActorBeginOverlap
  (params (OtherActor :type Actor%20Object%20Reference))
  (|CallParentFunction OtherActor) ; This node is disabled and will not be called.\nDrag off pins to build functionality.
)

(event EventTick
  (params (DeltaSeconds :type Float%20%28single-precision%29))
  (|CallParentFunction DeltaSeconds) ; This node is disabled and will not be called.\nDrag off pins to build functionality.
)

(event EventOnSelectedTileChanged
  (params (SelectedTile :type Tile%20BP%20Object%20Reference))
  (bind _position (Default|TileCenterPosition (Variables|Default|GetLevelManagerRef) (Variables|/Game/Blueprint/TileBP.TileBP_C|GetCoord SelectedTile)))
  (Rendering|Debug|DrawDebugSphere _position 5e+01 12 "(R=1.000000,G=0.000000,B=0.756083,A=1.000000)" 2e+01))

(fn ConstructionScript
  (|CallParentFunction))

(fn UpdateWidget
  (bind _levelmanagerref (Variables|Default|GetLevelManagerRef))
  (bind _tilemap (Variables|/Game/Blueprint/LevelManager.LevelManager_C|GetTileMap _levelmanagerref))
  (|CallParentFunction)
  (if (Variables|Default|GetIsActive)
    (bind _outactors (Actor|GetAllActorsOfClass "/Game/Blueprint/Enemies/EnemyBaseBP.EnemyBaseBP_C"))
    (for _array_element _outactors
      (Utilities|Array|Add (LocalVariables|GetValidCoord) (Variables|/Game/Blueprint/Enemies/EnemyBaseBP.EnemyBaseBP_C|GetPosition _array_element)))
    (Default|ClearTilesSelectable _tilemap)
    (Default|SetTilesSelectable _tilemap (LocalVariables|GetValidCoord))
    (bind _tile (Default|GetTile _tilemap))
    (Default|SetSelectable _tile "NewEnumerator2")
    (return false)
    (else
      (Default|ClearTilesSelectable (Variables|/Game/Blueprint/LevelManager.LevelManager_C|GetTileMap (Variables|Default|GetLevelManagerRef))))))